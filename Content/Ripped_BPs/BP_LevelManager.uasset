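; BP_LevelManager procedurally generates a level at BeginPlay: a spawn room, a random-length chain of rooms, then a boss room.
; Each step offsets the next room by a fixed grid distance along +Y, +X or -X, based on a random direction.
; Opposite sideways turns are rerolled so the path never doubles back.
; Each room receives its neighbouring directions to build entrances, and regular rooms also generate enemies.
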(event `self.ReceiveBeginPlay`
  (bind (_spawnlocation_x _spawnlocation_y _spawnlocation_z) (`KismetMathLibrary.BreakVector` (`self.SpawnLocation`)))
  (bind (_spawnlocation_x_2 _spawnlocation_y_2 _spawnlocation_z_2) (`KismetMathLibrary.BreakVector` (`self.SpawnLocation`)))
  (bind (_spawnlocation_x_3 _spawnlocation_y_3 _spawnlocation_z_3) (`KismetMathLibrary.BreakVector` (`self.SpawnLocation`)))
  (bind (_spawnlocation_x_4 _spawnlocation_y_4 _spawnlocation_z_4) (`KismetMathLibrary.BreakVector` (`self.SpawnLocation`)))
  (bind (_spawnlocation_x_5 _spawnlocation_y_5 _spawnlocation_z_5) (`KismetMathLibrary.BreakVector` (`self.SpawnLocation`)))
  (bind (_spawnlocation_x_6 _spawnlocation_y_6 _spawnlocation_z_6) (`KismetMathLibrary.BreakVector` (`self.SpawnLocation`)))
  (bind _returnvalue (`SceneComponent.GetRelativeTransform` (`self.DefaultSceneRoot`)))
  (`|SpawnActorFromClass` "/Game/Ripped_BPs/BP_SpawnRoom.BP_SpawnRoom_C" (`SceneComponent.GetRelativeTransform` (`self.DefaultSceneRoot`)) "Undefined" "OverrideRootScale" null null)
  (set `self.SpawnLocation` (`KismetMathLibrary.MakeVector` (.x (.location _returnvalue)) (+ (.y (.location _returnvalue)) 0.0) (.z (.location _returnvalue))))
  (for _index (range (+ (`KismetMathLibrary.RandomIntegerInRange` 5 10) 1))
    (set `self.GenCounter` _index)
    (switch `int` (`self.NextRoomVar`)
      (:`Default`
        (set `self.SpawnLocation` (`KismetMathLibrary.MakeVector` _spawnlocation_x (+ _spawnlocation_y 1500.0) _spawnlocation_z) :!label _label))
      (:`0`
        (goto _label))
      (:`1`
        (set `self.SpawnLocation` (`KismetMathLibrary.MakeVector` (+ _spawnlocation_x_2 1500.0) _spawnlocation_y_2 _spawnlocation_z_2)))
      (:`2`
        (set `self.SpawnLocation` (`KismetMathLibrary.MakeVector` (+ _spawnlocation_x_3 -1500.0) _spawnlocation_y_3 _spawnlocation_z_3))))
    (bind _returnvalue_2 (`|SpawnActorFromClass` "/Game/Ripped_BPs/BP_Room.BP_Room_C" (`KismetMathLibrary.MakeTransform` (`self.SpawnLocation`)) "Undefined" "OverrideRootScale" null null))
    (set `/Game/Ripped_BPs/BP_Room.GenerationCounter` (`self.GenCounter`) _returnvalue_2)
    (set `/Game/Ripped_BPs/BP_Room.PrevRoomType` (`self.NextRoomVar`) _returnvalue_2)
    (set `self.PrevRoomVar` (`self.NextRoomVar`))
    (set `self.NextRoomVar` (`KismetMathLibrary.RandomIntegerInRange` 0 2))
    (if (== (`self.PrevRoomVar`) 1) :!label _label_2
      (if (== (`self.NextRoomVar`) 2)
        (set `self.NextRoomVar` (`KismetMathLibrary.RandomIntegerInRange` 0 2))
        (goto _label_2)
        (else
          _))
      (elif (== (`self.PrevRoomVar`) 2)
        (if (== (`self.NextRoomVar`) 1)
          (set `self.NextRoomVar` (`KismetMathLibrary.RandomIntegerInRange` 0 2))
          (goto _label_2)
          (else
            _))))
    (set `/Game/Ripped_BPs/BP_Room.NextRoomType` (`self.NextRoomVar`) _returnvalue_2)
    (`/Game/Ripped_BPs/BP_Room.Build Entrance` _returnvalue_2)
    (`/Game/Ripped_BPs/BP_Room.GenerateEnemies` _returnvalue_2))
  (switch `int` (`self.NextRoomVar`)
    (:`Default`
      (set `self.SpawnLocation` (`KismetMathLibrary.MakeVector` _spawnlocation_x_5 (+ _spawnlocation_y_5 1500.0) _spawnlocation_z_5) :!label _label_3))
    (:`0`
      (goto _label_3))
    (:`1`
      (set `self.SpawnLocation` (`KismetMathLibrary.MakeVector` (+ _spawnlocation_x_6 1500.0) _spawnlocation_y_6 _spawnlocation_z_6)))
    (:`2`
      (set `self.SpawnLocation` (`KismetMathLibrary.MakeVector` (+ _spawnlocation_x_4 -1500.0) _spawnlocation_y_4 _spawnlocation_z_4))))
  (bind _returnvalue_3 (`|SpawnActorFromClass` "/Game/Ripped_BPs/BP_BossRoom.BP_BossRoom_C" (`KismetMathLibrary.MakeTransform` (`self.SpawnLocation`)) "Undefined" "OverrideRootScale" null null))
  (set `/Game/Ripped_BPs/BP_BossRoom.PrevRoomType` (`self.NextRoomVar`) _returnvalue_3)
  (`/Game/Ripped_BPs/BP_BossRoom.Build Entrance` _returnvalue_3))

(fn `UserConstructionScript`)
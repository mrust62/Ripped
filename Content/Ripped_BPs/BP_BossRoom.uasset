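; Boss room actor for a generated level, with events that open its entrance and spawn enemies.
; BuildEntrance destroys the left, back or front entrance component based on PrevRoomType; the branches that would also open an exit by NextRoomType are mostly disconnected.
; GenerateEnemies scatters BP_Enemy actors randomly around the room root at a fixed height, scaling the count with GenerationCounter up to a cap.
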(event `GenerateEnemies`
  (bind _generationcounter (`self.GenerationCounter`))
  (bind _returnvalue (`SceneComponent.GetRelativeTransform` (`self.DefaultSceneRoot`)))
  (if (< _generationcounter 4)
    (for _ (range (+ _generationcounter 1))
      (`|SpawnActorFromClass` "/Game/Ripped_BPs/BP_Enemy.BP_Enemy_C" (`KismetMathLibrary.MakeTransform` (`KismetMathLibrary.MakeVector` (+ (.x (.location _returnvalue)) (`KismetMathLibrary.RandomFloatInRange` -600.0 600.0)) (+ (.y (.location _returnvalue)) (`KismetMathLibrary.RandomFloatInRange` -600.0 600.0)) 100.0)) "AdjustIfPossibleButAlwaysSpawn" "OverrideRootScale" null null :!label _label))
    (else
      (for _ (range 5)
        (goto _label)))))

(event `Build Entrance`
  (switch `int` (`self.PrevRoomType`)
    (:`0`
      (switch `int` (`self.NextRoomType`)
        (:`0`
          (`ActorComponent.K2_DestroyComponent` (`self.LeftEntrance`)))
        (:`1`
          (`ActorComponent.K2_DestroyComponent` (`self.LeftEntrance`)))
        (:`2`
          (`ActorComponent.K2_DestroyComponent` (`self.LeftEntrance`)))))
    (:`1`
      (`ActorComponent.K2_DestroyComponent` (`self.BackEntrance`)))
    (:`2`
      (`ActorComponent.K2_DestroyComponent` (`self.FrontEntrance`)))))

(fn `UserConstructionScript`)
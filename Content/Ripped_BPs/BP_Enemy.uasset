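; BP_Enemy is an enemy actor that opens a combat screen when something overlaps its sphere.
; On first overlap it creates WT_EnemyCombat, copies in its own HP and that of BP_FirstPersonCharacter, then shows the cursor.
; Ending an actor overlap removes all widgets and hides the cursor.
; UIGenerated guards creation and is never reset here, and neither overlap event checks which actor triggered it.
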(event `self.Sphere.OnComponentBeginOverlap`
  (params (OverlappedComponent :type "PrimitiveComponent Object Reference") (OtherActor :type "Actor Object Reference") (OtherComp :type "PrimitiveComponent Object Reference") (OtherBodyIndex :type Integer) (bFromSweep :type Boolean) (SweepResult :type "HitResult Structure (by ref)"))
  (if (not (`self.UI Generated?`))
    (bind _returnvalue (`GameplayStatics.GetActorOfClass` "/Game/FirstPerson/Blueprints/BP_FirstPersonCharacter.BP_FirstPersonCharacter_C"))
    (bind _returnvalue_2 (`|CreateWidget` "/Game/WT_EnemyCombat.WT_EnemyCombat_C" (`GameplayStatics.GetPlayerController` 0)))
    (set `/Game/WT_EnemyCombat.EnemyHP` (`self.EnemyHP`) _returnvalue_2)
    (set `/Game/WT_EnemyCombat.MaxEnemyHP` (`self.EnemyMaxHP`) _returnvalue_2)
    (set `/Game/WT_EnemyCombat.PlayerHP` (`/Game/FirstPerson/Blueprints/BP_FirstPersonCharacter.PlayerHP` _returnvalue) _returnvalue_2)
    (set `/Game/WT_EnemyCombat.MaxPlayerHP` (`/Game/FirstPerson/Blueprints/BP_FirstPersonCharacter.PlayerMaxHP` _returnvalue) _returnvalue_2)
    (`UserWidget.AddToViewport` _returnvalue_2 0)
    (set `PlayerController.bShowMouseCursor` true (`GameplayStatics.GetPlayerController` 0))
    (set `self.UI Generated?` true)))

(event `self.ReceiveActorEndOverlap`
  (params (OtherActor :type "Actor Object Reference"))
  (`WidgetLayoutLibrary.RemoveAllWidgets`)
  (set `PlayerController.bShowMouseCursor` false (`GameplayStatics.GetPlayerController` 0)))

(fn `UserConstructionScript`)
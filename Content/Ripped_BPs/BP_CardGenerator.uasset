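; Card generator for a deck-building game that builds the player's starting deck and creates new cards to choose from.
; BeginPlay fills a fixed deck of attack, defense, heal and scrap cards and assigns it to BP_FirstPersonCharacter.
; GenerateNewCards rolls three random-type cards scaled to DefeatedEnemyLVL and shows them in WT_AddANewCard.
; Each card is a NewCardTemplate widget, with per-type functions setting its value, cost, text and art.
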(event `GenerateNewCards`
  (bind _returnvalue (+ (`self.DefeatedEnemyLVL`) 1))
  (bind _returnvalue_2 (/ _returnvalue 2))
  (for _ (range 3)
    (bind _returnvalue_3 (`|CreateWidget` "/Game/NewCardTemplate.NewCardTemplate_C"))
    (switch `int` (`KismetMathLibrary.RandomIntegerInRange` 0 3)
      (:`0`
        (bind _new_generated_card (`self.ATK Card` _returnvalue _returnvalue_2 _returnvalue_3))
        (set `self.ManipulatedCard` _new_generated_card))
      (:`1`
        (bind _newgeneratedcard (`self.DEF Card` _returnvalue _returnvalue_2 _returnvalue_3))
        (set `self.ManipulatedCard` _newgeneratedcard))
      (:`2`
        (bind _newgeneratedcard_2 (`self.HEAL Card` _returnvalue _returnvalue_2 _returnvalue_3))
        (set `self.ManipulatedCard` _newgeneratedcard_2))
      (:`3`
        (bind _newgeneratedcard_3 (`self.SCRP Card` _returnvalue 0 _returnvalue_3))
        (set `self.ManipulatedCard` _newgeneratedcard_3)))
    (set `/Game/NewCardTemplate.Active?` false (`self.ManipulatedCard`))
    (`KismetArrayLibrary.Array_Add` (`self.CardsForSelection`) (`self.ManipulatedCard`)))
  (bind _returnvalue_4 (`|CreateWidget` "/Game/WT_AddANewCard.WT_AddANewCard_C" (`GameplayStatics.GetPlayerController` 0)))
  (set `self.AddWT` _returnvalue_4)
  (`Widget.RemoveFromParent` _returnvalue_4)
  (set `/Game/WT_AddANewCard.CardsToChooseFrom` (`self.CardsForSelection`) (`self.AddWT`))
  (`UserWidget.AddToViewport` (`self.AddWT`) 0)
  (set `self.CardsForSelection` (`self.VOID`)))

(event `self.ReceiveBeginPlay`
  ;[1 1 1] Generate 4 Basic Attacks
  (for _ (range 4)
    (bind _returnvalue (`|CreateWidget` "/Game/NewCardTemplate.NewCardTemplate_C"))
    (bind _new_generated_card (`self.ATK Card` 1 1 _returnvalue))
    (`KismetArrayLibrary.Array_Add` (`self.GeneratedDeck`) _new_generated_card))
  ;[1 1 1] Generate 4 Basic Defense
  (for _ (range 4)
    (bind _returnvalue_2 (`|CreateWidget` "/Game/NewCardTemplate.NewCardTemplate_C"))
    (bind _newgeneratedcard (`self.DEF Card` 1 1 _returnvalue_2))
    (`KismetArrayLibrary.Array_Add` (`self.GeneratedDeck`) _newgeneratedcard))
  ;[1 1 1] Generate 4 Basic Heal
  (for _ (range 4)
    (bind _returnvalue_3 (`|CreateWidget` "/Game/NewCardTemplate.NewCardTemplate_C"))
    (bind _newgeneratedcard_2 (`self.HEAL Card` 1 1 _returnvalue_3))
    (`KismetArrayLibrary.Array_Add` (`self.GeneratedDeck`) _newgeneratedcard_2))
  ;[1 1 1] Generate 3 Basic Scraps
  (for _ (range 3)
    (bind _returnvalue_4 (`|CreateWidget` "/Game/NewCardTemplate.NewCardTemplate_C"))
    (bind _newgeneratedcard_3 (`self.SCRP Card` 1 0 _returnvalue_4))
    (`KismetArrayLibrary.Array_Add` (`self.GeneratedDeck`) _newgeneratedcard_3))
  ;[1 1 1] Generate 3 Big Attacks
  (for _ (range 3)
    (bind _returnvalue_5 (`|CreateWidget` "/Game/NewCardTemplate.NewCardTemplate_C"))
    (bind _new_generated_card_2 (`self.ATK Card` 3 2 _returnvalue_5))
    (`KismetArrayLibrary.Array_Add` (`self.GeneratedDeck`) _new_generated_card_2))
  (bind _asbp_first_person_character (cast `/Game/FirstPerson/Blueprints/BP_FirstPersonCharacter` (`GameplayStatics.GetPlayerCharacter` 0)))
  (set `/Game/FirstPerson/Blueprints/BP_FirstPersonCharacter.PlayerDeck` (`self.GeneratedDeck`) _asbp_first_person_character))

(fn `ATK Card`
  (params (LVL :type Integer) (Cost :type Integer) (NewCardElement :type "/Game/NewCardTemplate Object Reference"))
  (returns (`New Generated Card` :type "/Game/NewCardTemplate Object Reference"))
  (locals (ModifiedCard :type "/Game/CardTemplate Object Reference") (`NEW ModifiedCard` :type "/Game/NewCardTemplate Object Reference"))
  (bind _new_modifiedcard (`local.NEW ModifiedCard`))
  (set `local.NEW ModifiedCard` NewCardElement)
  (set `/Game/NewCardTemplate.CardValue` (+ (* LVL 3) 1) _new_modifiedcard)
  (set `/Game/NewCardTemplate.CardType` 1 _new_modifiedcard)
  (set `/Game/NewCardTemplate.CardCost` Cost _new_modifiedcard)
  (`TextBlock.SetText` (`/Game/NewCardTemplate.BEFORETXT` _new_modifiedcard) "Deal ")
  (`TextBlock.SetText` (`/Game/NewCardTemplate.AFTERTXT` _new_modifiedcard) " Damage")
  (`Image.SetBrush` (`/Game/NewCardTemplate.CardArt` _new_modifiedcard) (make `SlateBrush` (32.0 32.0) (struct) (struct :`SpecifiedColor` (struct :`R` 1.0 :`G` 1.0 :`B` 1.0 :`A` 1.0) :`ColorUseRule` "UseColor_Specified") (struct :`CornerRadii` (struct :`W` 1.0) :`Color` (struct :`SpecifiedColor` (struct) :`ColorUseRule` "UseColor_Specified") :`RoundingType` "HalfHeightRadius") "/Game/Ripped_Art/CardArtATK.CardArtATK"))
  (`Image.SetBrush` (`/Game/NewCardTemplate.CardBG` _new_modifiedcard) (make `SlateBrush` (32.0 32.0) (struct) (struct :`SpecifiedColor` (struct :`R` 1.0 :`G` 1.0 :`B` 1.0 :`A` 1.0) :`ColorUseRule` "UseColor_Specified") (struct :`CornerRadii` (struct :`W` 1.0) :`Color` (struct :`SpecifiedColor` (struct) :`ColorUseRule` "UseColor_Specified") :`RoundingType` "HalfHeightRadius") "/Game/Ripped_Art/CardArtBorderB.CardArtBorderB"))
  (return (`local.NEW ModifiedCard`)))

(fn `DEF Card`
  (params (LVL :type Integer) (Cost :type Integer) (NewCardElement :type "/Game/NewCardTemplate Object Reference"))
  (returns (NewGeneratedCard :type "/Game/NewCardTemplate Object Reference"))
  (locals (ModifiedCard :type "/Game/CardTemplate Object Reference") (NewModifiedCard :type "/Game/NewCardTemplate Object Reference"))
  (bind _newmodifiedcard (`local.NewModifiedCard`))
  (set `local.NewModifiedCard` NewCardElement)
  (set `/Game/NewCardTemplate.CardValue` (+ (* LVL 3) 1) _newmodifiedcard)
  (set `/Game/NewCardTemplate.CardType` 2 _newmodifiedcard)
  (set `/Game/NewCardTemplate.CardCost` Cost _newmodifiedcard)
  (`TextBlock.SetText` (`/Game/NewCardTemplate.BEFORETXT` _newmodifiedcard) "Gain ")
  (`TextBlock.SetText` (`/Game/NewCardTemplate.AFTERTXT` _newmodifiedcard) " Shield")
  (`Image.SetBrush` (`/Game/NewCardTemplate.CardArt` _newmodifiedcard) (make `SlateBrush` (32.0 32.0) (struct) (struct :`SpecifiedColor` (struct :`R` 1.0 :`G` 1.0 :`B` 1.0 :`A` 1.0) :`ColorUseRule` "UseColor_Specified") (struct :`CornerRadii` (struct :`W` 1.0) :`Color` (struct :`SpecifiedColor` (struct) :`ColorUseRule` "UseColor_Specified") :`RoundingType` "HalfHeightRadius") "/Game/Ripped_Art/CardArtDEF.CardArtDEF"))
  (`Image.SetBrush` (`/Game/NewCardTemplate.CardBG` _newmodifiedcard) (make `SlateBrush` (32.0 32.0) (struct) (struct :`SpecifiedColor` (struct :`R` 1.0 :`G` 1.0 :`B` 1.0 :`A` 1.0) :`ColorUseRule` "UseColor_Specified") (struct :`CornerRadii` (struct :`W` 1.0) :`Color` (struct :`SpecifiedColor` (struct) :`ColorUseRule` "UseColor_Specified") :`RoundingType` "HalfHeightRadius") "/Game/Ripped_Art/CardArtBorderC.CardArtBorderC"))
  (return (`local.NewModifiedCard`)))

(fn `HEAL Card`
  (params (LVL :type Integer) (Cost :type Integer) (NEWCardElement :type "/Game/NewCardTemplate Object Reference"))
  (returns (NEWGeneratedCard :type "/Game/NewCardTemplate Object Reference"))
  (locals (ModifiedCard :type "/Game/CardTemplate Object Reference") (NewModifiedCard :type "/Game/NewCardTemplate Object Reference"))
  (bind _newmodifiedcard (`local.NewModifiedCard`))
  (set `local.NewModifiedCard` NEWCardElement)
  (set `/Game/NewCardTemplate.CardValue` (* LVL 2) _newmodifiedcard)
  (set `/Game/NewCardTemplate.CardType` 3 _newmodifiedcard)
  (set `/Game/NewCardTemplate.CardCost` Cost _newmodifiedcard)
  (`TextBlock.SetText` (`/Game/NewCardTemplate.BEFORETXT` _newmodifiedcard) "Heal ")
  (`TextBlock.SetText` (`/Game/NewCardTemplate.AFTERTXT` _newmodifiedcard) " Health")
  (`Image.SetBrush` (`/Game/NewCardTemplate.CardArt` _newmodifiedcard) (make `SlateBrush` (32.0 32.0) (struct) (struct :`SpecifiedColor` (struct :`R` 1.0 :`G` 1.0 :`B` 1.0 :`A` 1.0) :`ColorUseRule` "UseColor_Specified") (struct :`CornerRadii` (struct :`W` 1.0) :`Color` (struct :`SpecifiedColor` (struct) :`ColorUseRule` "UseColor_Specified") :`RoundingType` "HalfHeightRadius") "/Game/Ripped_Art/CardArtHEAL.CardArtHEAL"))
  (`Image.SetBrush` (`/Game/NewCardTemplate.CardBG` _newmodifiedcard) (make `SlateBrush` (32.0 32.0) (struct) (struct :`SpecifiedColor` (struct :`R` 1.0 :`G` 1.0 :`B` 1.0 :`A` 1.0) :`ColorUseRule` "UseColor_Specified") (struct :`CornerRadii` (struct :`W` 1.0) :`Color` (struct :`SpecifiedColor` (struct) :`ColorUseRule` "UseColor_Specified") :`RoundingType` "HalfHeightRadius") "/Game/Ripped_Art/CardArtBorderA.CardArtBorderA"))
  (return (`local.NewModifiedCard`)))

(fn `SCRP Card`
  (params (LVL :type Integer) (Cost :type Integer) (NewCardElement :type "/Game/NewCardTemplate Object Reference"))
  (returns (NewGeneratedCard :type "/Game/NewCardTemplate Object Reference"))
  (locals (ModifiedCard :type "/Game/CardTemplate Object Reference") (NewModifedCard :type "/Game/NewCardTemplate Object Reference"))
  (bind _newmodifedcard (`local.NewModifedCard`))
  (set `local.NewModifedCard` NewCardElement)
  (set `/Game/NewCardTemplate.CardValue` (+ (/ LVL 4) 1) _newmodifedcard)
  (set `/Game/NewCardTemplate.CardType` 4 _newmodifedcard)
  (set `/Game/NewCardTemplate.CardCost` Cost _newmodifedcard)
  (`TextBlock.SetText` (`/Game/NewCardTemplate.BEFORETXT` _newmodifedcard) "Gain ")
  (`TextBlock.SetText` (`/Game/NewCardTemplate.AFTERTXT` _newmodifedcard) " Scrap")
  (`Image.SetBrush` (`/Game/NewCardTemplate.CardArt` _newmodifedcard) (make `SlateBrush` (32.0 32.0) (struct) (struct :`SpecifiedColor` (struct :`R` 1.0 :`G` 1.0 :`B` 1.0 :`A` 1.0) :`ColorUseRule` "UseColor_Specified") (struct :`CornerRadii` (struct :`W` 1.0) :`Color` (struct :`SpecifiedColor` (struct) :`ColorUseRule` "UseColor_Specified") :`RoundingType` "HalfHeightRadius") "/Game/Ripped_Art/CardArtENG.CardArtENG"))
  (`Image.SetBrush` (`/Game/NewCardTemplate.CardBG` _newmodifedcard) (make `SlateBrush` (32.0 32.0) (struct) (struct :`SpecifiedColor` (struct :`R` 1.0 :`G` 1.0 :`B` 1.0 :`A` 1.0) :`ColorUseRule` "UseColor_Specified") (struct :`CornerRadii` (struct :`W` 1.0) :`Color` (struct :`SpecifiedColor` (struct) :`ColorUseRule` "UseColor_Specified") :`RoundingType` "HalfHeightRadius") "/Game/Ripped_Art/CardArtBorderD.CardArtBorderD"))
  (return (`local.NewModifedCard`)))

(fn `UserConstructionScript`)